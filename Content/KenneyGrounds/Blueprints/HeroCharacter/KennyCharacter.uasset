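; Paper2D side-scrolling player character that moves along X, jumps, and turns by setting controller yaw.
; The MoveRight axis event also calls UpdateAnimation, which reduces velocity to 0 or 1 and sets the sprite's flipbook.
; AnimationState picks the flipbook through walk, idle, then jump checks, so the speed checks always win over Jump.
; Damage is a stub that only prints a debug string.
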(event Custom|UpdateAnimation
  ;[1 1 1] Handles Animations
  (Variables|Default|SetSpeed (Math|Conversions|ToFloat(Boolean) (> (Math|Vector|VectorLength (Transformation|GetVelocity)) 0.0)))
  (bind _outputflipbook (CallFunction|AnimationState (Variables|Default|GetSpeed) (Variables|Default|GetIsJumping)))
  (Sprite|SetFlipbook (Variables|Default|GetSprite) _outputflipbook))

(event Custom|Damage
  (Development|PrintString "laptop"))

(event Input|ActionEvents|InputActionJump
  ;[0.5 0.9 1] Jumping
  (:Pressed
    (Character|Jump)))

(event Input|AxisEvents|InputAxisMoveRight
  (params (AxisValue :type Float%20%28single-precision%29))
  ;[1 1 1] Movement
  (Pawn|Input|AddMovementInput "1.000000, 0, 0" AxisValue false)
  (CallFunction|UpdateAnimation)
  (Math|Float|CompareFloat AxisValue 0.0
    (:>
      (Pawn|SetControlRotation (Pawn|GetController) (Class|KismetMathLibrary|MakeRot 0.0 0.0 0.0)))
    (:<
      (Pawn|SetControlRotation (Pawn|GetController) (Class|KismetMathLibrary|MakeRot 0.0 1.8e+02 0.0)))))

(fn ConstructionScript)

(fn AnimationState
  (params (Speed :type Float%20%28single-precision%29) (Jumping :type Boolean))
  (Utilities|FlowControl|Sequence
    (:then_0
      ;[1 1 1] Store all local variables
      (LocalVariables|SetlocalSpeed Speed)
      (LocalVariables|SetlocalIsJumping Jumping))
    (:then_1
      (|CheckforWalking
        (:then
          (Variables|Default|SetAnimStateEnum "NewEnumerator2"))
        (:else
          (|CheckforIdling
            (:then
              (Variables|Default|SetAnimStateEnum "NewEnumerator0"))
            (:else
              (|CheckforJumping)
              (Variables|Default|SetAnimStateEnum "NewEnumerator1")))))
      (return (Utilities|Select :Index (Variables|Default|GetAnimStateEnum) :NewEnumerator0 (Variables|Animations|GetIdleFlipbook) :NewEnumerator1 (Variables|Animations|GetJumpFlipbook) :NewEnumerator2 (Variables|Animations|GetWalkFlipbook))))))