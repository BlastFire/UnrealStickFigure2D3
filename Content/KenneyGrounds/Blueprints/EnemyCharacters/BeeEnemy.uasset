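; Bee enemy that damages the player's KennyCharacter whenever it overlaps it.
; The construction script sets the movement component's initial speed from the absolute value of Speed.
; A BeeMovement timeline is set up to add a wave-like vertical offset scaled by WaveAmount, but nothing in the graph starts it.
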(event `self.ReceiveActorBeginOverlap`
  (params (OtherActor :type "Actor Object Reference"))
  ;[1 1 1] Collision with the player
  (bind _askenny_character (cast `/Game/KenneyGrounds/Blueprints/HeroCharacter/KennyCharacter` OtherActor))
  (`/Game/KenneyGrounds/Blueprints/HeroCharacter/KennyCharacter.Damage` _askenny_character))

(fn `UserConstructionScript`
  ;[0.6767 1 0.5658] Change the initial speed
  (set `ProjectileMovementComponent.InitialSpeed` (`KismetMathLibrary.Abs` (`self.Speed`)) (`self.Movement`)))