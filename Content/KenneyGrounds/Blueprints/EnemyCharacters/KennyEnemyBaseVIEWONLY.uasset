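; KennyEnemyBaseVIEWONLY is a 2D Paper2D enemy base that moves by projectile movement.
; The construction script adds the EnemySprite, sizes the collision sphere to half its bounds radius and sets initial speed from absolute Speed.
; FaceLeft yaws the sprite around and points velocity along negative X.
; Overlap handling is only debug prints that report whether the other actor is a KennyCharacter.
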(event `self.ReceiveActorBeginOverlap`
  (params (OtherActor :type "Actor Object Reference"))
  (cast `/Game/KenneyGrounds/Blueprints/HeroCharacter/KennyCharacter` OtherActor
    (:`then`
      (`KismetSystemLibrary.PrintString` "Collision"))
    (:`CastFailed`
      (`KismetSystemLibrary.PrintString` "Fail"))))

(fn `UserConstructionScript`
  (bind _returnvalue (`AddComponent|PaperSpriteComponent_437`))
  (set `self.Sprite` _returnvalue)
  (`PaperSpriteComponent.SetSprite` _returnvalue (`self.EnemySprite`))
  (`SphereComponent.SetSphereRadius` (`self.Collision`) (* (`.SphereRadius` (`KismetSystemLibrary.GetComponentBounds` (`self.Sprite`))) 0.5) true)
  (set `ProjectileMovementComponent.InitialSpeed` (`KismetMathLibrary.Abs` (`self.Speed`)) (`self.ProjectileMovement1`))
  (if (`self.FaceLeft`)
    (`SceneComponent.K2_AddRelativeRotation` (`self.Sprite`) (`KismetMathLibrary.MakeRot` 0.0 180.0) false)
    (set `MovementComponent.Velocity` (-1.0 0.0 0.0) (`self.ProjectileMovement1`))))